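; GameCharacter is a character Blueprint that kills other GameCharacters on contact with its KillBox component.
; When another GameCharacter overlaps the box, it calls Kill, ignoring itself and other actor types.
; Kill calls Killed on the victim with this character as the killer, and the victim destroys itself without using that reference.
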(event `self.KillBox.OnComponentBeginOverlap`
  (params (OtherActor :type "Actor Object Reference") (OtherComp :type "PrimitiveComponent Object Reference") (OtherBodyIndex :type Integer) (bFromSweep :type Boolean) (SweepResult :type "EngineTypes.HitResult Structure (by ref)"))
  ;[1 1 1] Check whether gamecharacter is not self.
  (bind _asgame_character (cast `/Game/Blueprints/Characters/GameCharacter` OtherActor))
  (if (!= _asgame_character self)
    ;[1 1 1] This character kills the other.
    (`self.Kill` self _asgame_character)))

(fn `Kill`
  (params (Killed :type "/Game/Blueprints/Characters/GameCharacter Object Reference"))
  ;[1 1 1] The other character is killed by this.
  (`self.Killed` Killed self))

(fn `Killed`
  (params (Killer :type "/Game/Blueprints/Characters/GameCharacter Object Reference"))
  (`self.K2_DestroyActor`))

(fn `UserConstructionScript`)