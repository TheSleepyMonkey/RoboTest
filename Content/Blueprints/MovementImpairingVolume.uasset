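; MovementImpairingVolume is a volume actor that changes a MyCharacter's MovementSpeed while it overlaps the volume.
; Begin overlap applies this volume's MovementModifier directly, replacing the current value without comparison.
; End overlap scans the volumes still overlapping player character 0, not necessarily the exiting character, and applies the lowest modifier below 1.0 to the exiting character, defaulting to 1.0.
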(event `self.ReceiveActorBeginOverlap`
  (params (OtherActor :type "Actor Object Reference"))
  ;[1 1 1] onbegin take new reduction
  (bind _asmy_character (cast `/Game/Blueprints/Characters/MyCharacter` OtherActor))
  (set `/Game/Blueprints/Characters/MyCharacter.movementSpeed` (`self.MovementModifier`) _asmy_character))

(event `self.ReceiveActorEndOverlap`
  (params (OtherActor :type "Actor Object Reference"))
  (bind _newspeed (`self.NewSpeed`))
  ;[1 1 1] Keep lowest
  (bind _asmy_character (cast `/Game/Blueprints/Characters/MyCharacter` OtherActor))
  (set `self.NewSpeed` 1.0)
  (for _array_element (`self.GetOverlappingActors` (`GameplayStatics.GetPlayerCharacter` 0) "MovementImpairingVolume_C")
    (bind _asmovement_impairing_volume (cast `/Game/Blueprints/MovementImpairingVolume` _array_element))
    (bind _movementmodifier (`/Game/Blueprints/MovementImpairingVolume.MovementModifier` _asmovement_impairing_volume))
    (`/Engine/EditorBlueprintResources/StandardMacros.CompareFloat` _movementmodifier _newspeed
      (:`<`
        (set `self.NewSpeed` _movementmodifier))))
  (set `/Game/Blueprints/Characters/MyCharacter.movementSpeed` _newspeed _asmy_character))

(fn `UserConstructionScript`)