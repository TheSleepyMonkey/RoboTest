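; EndZone is a level-finish trigger that ends play and opens the finish menu when any actor overlaps it.
; The overlap disables player input, stops movement, pauses the game and shows a FinishMenu widget that receives the NewLevel value as its next level.
; An unconnected timeline would lerp the player through MoveToCenter to the zone's X, zero Y and its own height before finishing.
; The falling check has no effect.
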(event `self.ReceiveActorBeginOverlap`
  (params (OtherActor :type "Actor Object Reference"))
  (bind _returnvalue (`Pawn.GetMovementComponent` (`GameplayStatics.GetPlayerPawn` 0)))
  (if (`NavMovementComponent.IsFalling` _returnvalue)
    _
    (else
      _))
  (`self.DisableInput` (`GameplayStatics.GetPlayerCharacter` 0) (`GameplayStatics.GetPlayerController` 0))
  (`MovementComponent.StopMovementImmediately` _returnvalue)
  (`GameplayStatics.SetGamePaused` true)
  (bind _returnvalue_2 (`|CreateWidget` "/Game/Blueprints/Menus/FinishMenu.FinishMenu_C"))
  (set `/Game/Blueprints/Menus/FinishMenu.NextLevel` (`self.NewLevel`) _returnvalue_2)
  (`UserWidget.AddToViewport` _returnvalue_2 0))

(fn `MoveToCenter`
  (params (NewParam :type "Float (double-precision)"))
  (bind _returnvalue (`GameplayStatics.GetPlayerPawn` 0))
  (bind _returnvalue_2 (`self.K2_GetActorLocation` _returnvalue))
  (`self.K2_SetActorRelativeLocation` _returnvalue (`KismetMathLibrary.VLerp` _returnvalue_2 (+ (* (`self.K2_GetActorLocation`) (1.0 0.0 0.0)) (* _returnvalue_2 (0.0 0.0 1.0))) NewParam) false))

(fn `UserConstructionScript`)