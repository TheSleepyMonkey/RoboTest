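; Lift Blueprint that moves a sprite back and forth between its origin and a configurable end location.
; A timeline scaled by travel time lerps the sprite, pausing at each end before running the opposite way.
; A safety collider flips the timeline direction when the player character overlaps it while the lift moves.
; The construction script applies the lift color and can preview the end location in the editor.
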(event `self.ReceiveBeginPlay`
  (`TimelineComponent.SetPlayRate` (`self.LiftTimeline`) (/ 1.0 (`self.TravelTimeSeconds`)))
  (set `self.TestEndLocation` false))

(event `self.SafetyCollider.OnComponentBeginOverlap`
  (params (OtherActor :type "Actor Object Reference") (OtherComp :type "PrimitiveComponent Object Reference") (OtherBodyIndex :type Integer) (bFromSweep :type Boolean) (SweepResult :type "EngineTypes.HitResult Structure (by ref)"))
  (bind _lifttimeline (`self.LiftTimeline`))
  (cast `/Game/Blueprints/Characters/MyCharacter` OtherActor)
  (if (`ActorComponent.IsActive` _lifttimeline)
    (if (`TimelineComponent.IsReversing` _lifttimeline)
      (bind (_direction _lerpalpha) (`Timeline|LiftTimeline` :!label _label)
        (:`Update`
          (`SceneComponent.K2_SetRelativeLocation` (`self.LiftSprite`) (`KismetMathLibrary.VLerp` (0.0 0.0 0.0) (`self.EndLocation`) _lerpalpha) false))
        (:`Finished`
          (`KismetSystemLibrary.Delay` (`self.StopDelay`))
          (switch `TimelineComponent.ETimelineDirection` _direction
            (:`Forward`
              (`self.LiftBackward`))
            (:`Backward`
              (`self.LiftForward`)))))
      (else
        (goto _label :!via `Reverse`)))))

(event `LiftForward`
  (goto _label :!via `PlayFromStart`))

(event `LiftBackward`
  (goto _label :!via `ReverseFromEnd`))

(fn `UserConstructionScript`
  (`SceneComponent.K2_SetRelativeLocation` (`KismetMathLibrary.SelectVector` (`self.EndLocation`) (0.0 0.0 0.0) (`self.TestEndLocation`)))
  (`PaperSpriteComponent.SetSpriteColor` (`self.LiftColor`)))