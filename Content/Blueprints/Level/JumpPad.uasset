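; Jump pad Blueprint that bounces any Character overlapping its TrampolineCollider.
; It stops the character's movement, then calls LaunchCharacter with a BounceSpeed vector rotated by the Root's relative rotation to follow the pad's tilt.
; The vector's X and Y read the movement velocity after the stop has zeroed it, so the launch runs along the pad's up axis.
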(event `self.TrampolineCollider.OnComponentBeginOverlap`
  (params (OtherActor :type "Actor Object Reference") (OtherComp :type "PrimitiveComponent Object Reference") (OtherBodyIndex :type Integer) (bFromSweep :type Boolean) (SweepResult :type "HitResult Structure (by ref)"))
  (bind _ascharacter (cast `Character` OtherActor))
  ;[1 1 1] Stop movement and set launch vector correctly.
  (`MovementComponent.StopMovementImmediately` _ascharacter)
  (`Character.LaunchCharacter` _ascharacter (`KismetMathLibrary.GreaterGreater_VectorRotator` (`KismetMathLibrary.MakeVector` (.x (`MovementComponent.Velocity` (`Pawn.GetMovementComponent` _ascharacter))) (.y (`MovementComponent.Velocity` (`Pawn.GetMovementComponent` _ascharacter))) (`self.BounceSpeed`)) (`SceneComponent.RelativeRotation` (`self.Root`))) false false))

(fn `UserConstructionScript`)