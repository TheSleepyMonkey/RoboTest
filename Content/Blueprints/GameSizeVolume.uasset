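; GameSizeVolume is a volume actor that sets the camera position limits of MyCharacter when the character overlaps it.
; On begin overlap, it casts the other actor to MyCharacter and writes the character's MinCameraPosition and MaxCameraPosition.
; GetMinMax derives both corners from the Box1 component's world bounds, using its origin and extent.
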(event `self.ReceiveActorBeginOverlap`
  (params (OtherActor :type "Actor Object Reference"))
  (bind _asmy_character (cast `/Game/Blueprints/Characters/MyCharacter` OtherActor))
  (bind (_min _max) (`self.GetMinMax`))
  (set `/Game/Blueprints/Characters/MyCharacter.MinCameraPosition` _min _asmy_character)
  (set `/Game/Blueprints/Characters/MyCharacter.MaxCameraPosition` _max _asmy_character))

(fn `GetMinMax`
  (returns (Min :type "Object.Vector Structure") (Max :type "Object.Vector Structure"))
  (bind (_origin _boxextent) (`KismetSystemLibrary.GetComponentBounds` (`self.Box1`)))
  (bind _returnvalue (- _origin _boxextent))
  (return _returnvalue (+ _returnvalue (* _boxextent 2.0))))

(fn `UserConstructionScript`)