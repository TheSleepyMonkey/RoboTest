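; AI controller that walks its controlled pawn steadily along the world X axis.
; Each tick it adds movement input only while the pawn's vertical velocity is exactly zero, which it treats as being on the ground.
; The MovesRight boolean converts to a +1 or -1 scale that sets the direction; nothing in this controller changes that flag.
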(event `self.ReceiveBeginPlay`)

(event `self.ReceiveTick`
  (params (DeltaSeconds :type "Float (single-precision)"))
  (bind _returnvalue (`self.K2_GetPawn`))
  ;[1 1 1] Is actor on the ground?
  (if (== 0.0 (.z (`self.GetVelocity` _returnvalue)))
    (`Pawn.AddMovementInput` _returnvalue (1.0 0.0 0.0) (`KismetMathLibrary.Conv_IntToDouble` (- (* (`KismetMathLibrary.Conv_BoolToInt` (`self.movesRight`)) 2) 1)) false)))

(fn `UserConstructionScript`)