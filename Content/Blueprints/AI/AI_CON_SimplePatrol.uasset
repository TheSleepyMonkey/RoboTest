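; AI controller that walks its pawn around a looping patrol route of linked PatrolPoint actors.
; On BeginPlay it spawns a StartPoint at the pawn's location, which SetDesiredPoint links to the supplied point, optionally moving immediately.
; Whenever Tick finds the pawn not moving, it moves to DesiredPoint and advances along NextPoint links.
; A chain without a next point gets linked back to StartPoint, closing the loop.
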(event `self.ReceiveBeginPlay`
  (bind _returnvalue (`|SpawnActorFromClass` "/Game/Blueprints/Level/PatrolPoint.PatrolPoint_C" (`KismetMathLibrary.Conv_VectorToTransform` (`self.K2_GetActorLocation` (`self.K2_GetPawn`))) true))
  (set `self.StartPoint` _returnvalue))

(event `Set Desired Point`
  (params (newPoint :type "/Game/Blueprints/Level/PatrolPoint Object Reference") (moveDirect :type Boolean :default false))
  (bind _nextpoint (`/Game/Blueprints/Level/PatrolPoint.NextPoint` (`self.DesiredPoint`)))
  (bind _output_get (set `self.DesiredPoint` newPoint))
  (set `/Game/Blueprints/Level/PatrolPoint.NextPoint` _output_get (`self.StartPoint`))
  (if moveDirect
    (`self.MoveToActor` (`self.DesiredPoint`) (`self.AcceptanceRadius`) :!label _label)
    ;[1 1 1] Set new desired position.
    (if (`KismetSystemLibrary.IsValid` _nextpoint)
      (set `self.DesiredPoint` _nextpoint)
      (else
        (bind _output_get_2 (set `/Game/Blueprints/Level/PatrolPoint.NextPoint` (`self.StartPoint`) (`self.DesiredPoint`)))
        (set `self.DesiredPoint` _output_get_2)))))

(event `self.ReceiveTick`
  (params (DeltaSeconds :type "Float (single-precision)"))
  (if (!= (`self.GetMoveStatus`) (enumliteral `PathFollowingComponent.EPathFollowingStatus` "Moving"))
    (goto _label)))

(fn `UserConstructionScript`)